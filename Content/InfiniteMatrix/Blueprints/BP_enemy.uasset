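; BP_enemy is an enemy obstacle that damages the player on contact and can be destroyed by bullets.
; Overlapping the player destroys the enemy mesh component, reduces health, updates the health bar, and triggers death and restart display at zero.
; Overlapping a bullet destroys both the bullet and the mesh component.
; RandomizeE randomly assigns the enemy mesh or none and scatters the root's relative location within fixed bounds.
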(event OnComponentBeginOverlap(enemy1)
  (params (OverlappedComponent :type Primitive%20Component%20Object%20Reference) (OtherActor :type Actor%20Object%20Reference) (OtherComp :type Primitive%20Component%20Object%20Reference) (OtherBodyIndex :type Integer) (bFromSweep :type Boolean) (SweepResult :type Hit%20Result%20Structure%20%28by%20ref%29))
  (bind _asbp_player (Utilities|Casting|CastToBP_Player OtherActor)
    (:then
      (Components|DestroyComponent (Variables|Default|Getenemy1))
      (bind _output_get (Variables|/Game/InfiniteMatrix/Blueprints/BP_Player.BP_Player_C|SetHealth _asbp_player (- (Variables|/Game/InfiniteMatrix/Blueprints/BP_Player.BP_Player_C|GetHealth _asbp_player) 3e+01)))
      (Default|Updatehealth (Variables|/Game/InfiniteMatrix/Blueprints/BP_Player.BP_Player_C|GetHealthbar _asbp_player) _output_get)
      (if (<= _output_get 0.0)
        (Variables|/Game/InfiniteMatrix/Blueprints/BP_Player.BP_Player_C|SetIsDead _asbp_player true)
        (Default|DisplayRestart _asbp_player)))
    (:CastFailed
      (bind _asbp_bullet (Utilities|Casting|CastToBP_Bullet OtherActor))
      (Actor|DestroyActor _asbp_bullet)
      (Components|DestroyComponent (Variables|Default|Getenemy1)))))

(event EventBeginPlay)

(event Collision|EventActorBeginOverlap
  (params (OtherActor :type Actor%20Object%20Reference)))

(event EventTick
  (params (DeltaSeconds :type Float%20%28single-precision%29)))

(fn ConstructionScript)

(fn RandomizeE
  (Components|StaticMesh|SetStaticMesh (Variables|Default|Getenemy1) (Utilities|Select :Index (Math|Random|RandomIntegerinRange 0 2) :Option%200 "/Game/InfiniteMatrix/Blueprints/SM_Enemy.SM_Enemy" :Option%201 0))
  (Transformation|SetRelativeLocation (Variables|Default|GetDefaultSceneRoot) (Math|Vector|MakeVector (Math|Random|RandomFloatinRange 9e+02 2.1e+03) (Math|Random|RandomFloatinRange -3e+02 3e+02) (Math|Random|RandomFloatinRange -2e+02 2e+02)) false false))